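; AI controller that drives a BP_Runner pawn by faking alternating left and right power inputs.
; On possess it caches the runner, and BeginPlay starts the first delayed input.
; Each simulated input flip-flops between the runner's left and right power calls, then schedules another timer with a random delay between the configured minimum and maximum.
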(event `self.ReceiveBeginPlay`
  (`self.Simulate Input with delay`))

(event `self.ReceivePossess`
  (params (PossessedPawn :type "Pawn Object Reference"))
  (bind _asbp_runner (cast `/Game/Blueprints/BP_Runner` PossessedPawn))
  (set `self.Owning Runner` _asbp_runner))

(event `Simulate Input`
  (`/Engine/EditorBlueprintResources/StandardMacros.FlipFlop`
    (:`A`
      (`/Game/Blueprints/BP_Runner.Simulate Power Left` (`self.Owning Runner`))
      (`self.Simulate Input with delay`))
    (:`B`
      (`/Game/Blueprints/BP_Runner.Simulate Power Right` (`self.Owning Runner`))
      (`self.Simulate Input with delay`))))

(fn `Simulate Input with delay`
  (`KismetSystemLibrary.K2_SetTimerDelegate` (`|CreateDelegate` :!event `Simulate Input`) (`KismetMathLibrary.RandomFloatInRange` (`self.Min Input Delay`) (`self.Max Input Delay`))))

(fn `UserConstructionScript`)